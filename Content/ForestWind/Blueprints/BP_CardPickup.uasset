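; BP_CardPickup is a world pickup that adds a card to the player's deck.
; On BeginPlay it looks up the first CurrentCard entry in its data table and shows that row on two card visual widget components.
; When BP_ThirdPersonCharacter overlaps its box, it adds the row to the deck obtained through a Game Instance interface message.
; It then shows a WBP_CardObtain popup of the card and destroys itself.
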(event `self.ReceiveBeginPlay`
  (bind (_datatable _rowname) (break `DataTableRowHandle` (`|GetArrayItem` (`.Cards_8_4589AA53415BAE79FE1775B9072DE680` (break `/Game/RLDB/Blueprints/Structs/FDeck` (`self.CurrentCard`))))))
  (bind _returnvalue (`|GetDataTableRow` _datatable _rowname)
    (:`then`
      (`|ExecutionSequence`
        (:`then_0`
          (bind _aswbp_card_visual_simple (cast `/Game/RLDB/Widgets/WBP_CardVisualSimple` (`WidgetComponent.GetWidget` (`self.Widget1`))))
          (`/Game/RLDB/Widgets/WBP_CardVisualSimple.UpdateVisual` _aswbp_card_visual_simple _returnvalue))
        (:`then_1`
          (bind _aswbp_card_visual_simple_2 (cast `/Game/RLDB/Widgets/WBP_CardVisualSimple` (`WidgetComponent.GetWidget` (`self.Widget`))))
          (`/Game/RLDB/Widgets/WBP_CardVisualSimple.UpdateVisual` _aswbp_card_visual_simple_2 _returnvalue))))))

(event `self.Box.OnComponentBeginOverlap`
  (params (OverlappedComponent :type "PrimitiveComponent Object Reference") (OtherActor :type "Actor Object Reference") (OtherComp :type "PrimitiveComponent Object Reference") (OtherBodyIndex :type Integer) (bFromSweep :type Boolean) (SweepResult :type "HitResult Structure (by ref)"))
  (cast `/Game/ForestWind/Blueprints/BP_ThirdPersonCharacter` OtherActor)
  (bind (_bsuccess _deck) (message `/Game/RLDB/Blueprints/Interfaces/BPI_CardGameInstance.GetDeckCreationsFromInstance` (`GameplayStatics.GetGameInstance`)))
  (`KismetArrayLibrary.Array_Add` _deck (stale `self.ReceiveBeginPlay` _returnvalue))
  (bind _returnvalue (`|CreateWidget` "/Game/ForestWind/UI/WBP_CardObtain.WBP_CardObtain_C"))
  (`/Game/RLDB/Widgets/WBP_CardVisualSimple.UpdateVisual` (`/Game/ForestWind/UI/WBP_CardObtain.WBP_CardVisualSimple` _returnvalue) (stale `self.ReceiveBeginPlay` _returnvalue))
  (`UserWidget.AddToViewport` _returnvalue 0)
  (`self.K2_DestroyActor`))

(fn `UserConstructionScript`)