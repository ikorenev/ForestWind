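; BP_Observer is an actor that acts as an AND gate between condition actors and the actors waiting on them.
; On BeginPlay it sets itself as each condition actor's Observer and maps that actor to false.
; Activate and Deactivate update the map, and when all values are true, Activate sends ActivateMessage to every ActorsRequestCondition entry.
; A Deactivate while Ready clears the flag and sends them DeactivateMessage.
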(event `self.ReceiveBeginPlay`
  (for _array_element (`self.ActorsForChangeCondition`)
    (set `/Game/ForestWind/Blueprints/BP_InteractObj.Observer` self _array_element)
    (`BlueprintMapLibrary.Map_Add` (`self.StatusActorsForChangeCondition`) _array_element)))

(event `self.ReceiveTick`
  (params (DeltaSeconds :type "Float (single-precision)")))

(event `/Game/ForestWind/Blueprints/BPI_Activate.Activate`
  (params (Obj :type "/Game/ForestWind/Blueprints/BP_InteractObj Object Reference"))
  (`BlueprintMapLibrary.Map_Add` (`self.StatusActorsForChangeCondition`) Obj true)
  (bind _values (`BlueprintMapLibrary.Map_Values` (`self.StatusActorsForChangeCondition`)))
  (for _array_element _values
    (if _array_element
      (set `self.Ready` true)
      (else
        (set `self.Ready` false)
        (break))))
  (if (`self.Ready`)
    (for _array_element_2 (`self.ActorsRequestCondition`)
      (message `/Game/ForestWind/Blueprints/BPI_Activate.Activate` _array_element_2 null))))

(event `/Game/ForestWind/Blueprints/BPI_Activate.Deactivate`
  (params (Obj :type "/Game/ForestWind/Blueprints/BP_InteractObj Object Reference"))
  (`BlueprintMapLibrary.Map_Add` (`self.StatusActorsForChangeCondition`) Obj)
  (if (`self.Ready`)
    (set `self.Ready` false)
    (for _array_element (`self.ActorsRequestCondition`)
      (message `/Game/ForestWind/Blueprints/BPI_Activate.Deactivate` _array_element null))))

(fn `UserConstructionScript`)