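; BP_Enemy is an enemy that starts an encounter when BP_ThirdPersonCharacter overlaps its Box.
; The overlap stores the player's location on the GameInstance, then looks up the Encounter data table row.
; If the row is found, it saves the game, sets the current encounter, records a done story encounter and opens the row's level, all GameInstance calls going through interface messages.
; A direct open of L_Battle is left unconnected.
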(event `self.CapsuleComponent.OnComponentHit`
  (params (HitComponent :type "PrimitiveComponent Object Reference") (OtherActor :type "Actor Object Reference") (OtherComp :type "PrimitiveComponent Object Reference") (NormalImpulse :type "Vector Structure") (Hit :type "HitResult Structure (by ref)")))

(event `self.Box.OnComponentBeginOverlap`
  (params (OverlappedComponent :type "PrimitiveComponent Object Reference") (OtherActor :type "Actor Object Reference") (OtherComp :type "PrimitiveComponent Object Reference") (OtherBodyIndex :type Integer) (bFromSweep :type Boolean) (SweepResult :type "HitResult Structure (by ref)"))
  (bind (_datatable _rowname) (break `DataTableRowHandle` (`self.Encounter`)))
  (bind _asbp_third_person_character (cast `/Game/ForestWind/Blueprints/BP_ThirdPersonCharacter` OtherActor))
  (message `/Game/RLDB/Blueprints/Interfaces/BPI_CardGameInstance.SavePosOnLevel` (`GameplayStatics.GetGameInstance`) (`self.K2_GetActorLocation` _asbp_third_person_character))
  (bind _returnvalue (`|GetDataTableRow` _datatable _rowname)
    (:`then`
      (message `/Game/RLDB/Blueprints/Interfaces/BPI_CardGameInstance.AttemptSaveGame` (`GameplayStatics.GetGameInstance`) "" false)
      (message `/Game/RLDB/Blueprints/Interfaces/BPI_CardGameInstance.SetCurrentEncounterInInstance` (`GameplayStatics.GetGameInstance`) _returnvalue)
      (message `/Game/RLDB/Blueprints/Interfaces/BPI_CardGameInstance.AddDoneStoryEncounterToInstance` (`GameplayStatics.GetGameInstance`) (struct))
      (`GameplayStatics.OpenLevel` (`KismetStringLibrary.Conv_StringToName` (`.Level_9_A25929C34E49E8B28275AF917100AE74` (break `/Game/RLDB/Blueprints/Structs/FEncounter` _returnvalue)))))))

(fn `UserConstructionScript`)