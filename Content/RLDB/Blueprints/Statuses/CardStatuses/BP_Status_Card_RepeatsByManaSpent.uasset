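; Card status that makes a card an X-cost spell: it costs all the player's mana (minimum 1) and repeats once per point beyond the first.
; While the card is in hand, it listens on the player's dispatcher hub for mana changes, unbinding on exit or pre-play.
; UpdateFromMana rewrites the mana cost rule and repetition count, then broadcasts that the card was modified.
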(event `self.ReceiveBeginPlay`
  (`parent.ReceiveBeginPlay`)
  (bind _asbp_card (cast `/Game/RLDB/Blueprints/Core/BP_Card` (`self.GetOwner`)))
  (set `self.OwningCard` _asbp_card)
  (`/Game/RLDB/Blueprints/Core/BP_DispatcherHubComponent.BindMultipleEventsToHub` (`.ReturnValue` (`self.GetOwnersDispatcherHub`)) self (struct :`GameplayTags` (struct :`(TagName` "Event.Card.EnterHand") :`(TagName` "Event.Card.ExitHand") :`(TagName` "Event.Card.PrePlay") :`(TagName` "Event.Card.ModifyInHand")))))

(event `/Game/RLDB/Blueprints/Interfaces/BPI_EventHolder.RunEvent`
  (params (EventTag :type "GameplayTag Structure") (CallingObject :type "Object Object Reference (by ref)") (bGlobal :type Boolean) (Payload :type "Object Object Reference (by ref)") (CallTags :type "GameplayTagContainer Structure (by ref)"))
  (`|SwitchGameplayTag` EventTag
    (:`Event.Card.EnterHand`
      (`/Game/RLDB/Blueprints/Core/BP_DispatcherHubComponent.BindEventToHub` (`/Game/RLDB/Blueprints/Core/BP_CardPlayer.BP_DispatcherHubComponent_Local` (`/Game/RLDB/Blueprints/Libraries/BPFL_Singletons.GetCardPlayerPure`)) self (struct :`TagName` "Event.PostModifyStatus"))
      (`self.UpdateFromMana` (`/Game/RLDB/Blueprints/Statuses/BP_Status.StatusValue` (`/Game/RLDB/Blueprints/Core/BP_CardPlayer.BP_Status_Mana` (`/Game/RLDB/Blueprints/Libraries/BPFL_Singletons.GetCardPlayerPure`)))))
    (:`Event.Card.ExitHand`
      (`/Game/RLDB/Blueprints/Core/BP_DispatcherHubComponent.UnbindEventFromHub` (`/Game/RLDB/Blueprints/Core/BP_CardPlayer.BP_DispatcherHubComponent_Local` (`/Game/RLDB/Blueprints/Libraries/BPFL_Singletons.GetCardPlayerPure`)) self (struct :`TagName` "Event.PostModifyStatus") :!label _label))
    (:`Event.Card.PrePlay`
      (goto _label))
    (:`Event.PostModifyStatus`
      (bind _asbp_status_mana (cast `/Game/RLDB/Blueprints/Statuses/BP_Status_Mana` CallingObject))
      (`self.UpdateFromMana` (`/Game/RLDB/Blueprints/Statuses/BP_Status.StatusValue` _asbp_status_mana)))
    (:`Event.Card.ModifyInHand`
      (bind _cardplayer (`/Game/RLDB/Blueprints/Libraries/BPFL_Singletons.GetCardPlayer`))
      (`self.UpdateFromMana` (`/Game/RLDB/Blueprints/Statuses/BP_Status.StatusValue` (`Actor.GetComponentByClass` _cardplayer "/Game/RLDB/Blueprints/Statuses/BP_Status_Mana.BP_Status_Mana_C"))))))

(fn `UpdateFromMana`
  (params (Mana :type Integer))
  (`/Game/RLDB/Blueprints/Core/BP_Card.SetUseRuleCost` (`self.OwningCard`) "/Game/RLDB/Blueprints/CardUseRules/BP_UseRule_StatCost.BP_UseRule_StatCost_C" "/Game/RLDB/Blueprints/Statuses/BP_Status_Mana.BP_Status_Mana_C" (`KismetMathLibrary.Max` Mana 1) "NewEnumerator0" true)
  (`/Game/RLDB/Blueprints/Core/BP_Card.SetCardRepetitions` (`self.OwningCard`) "NewEnumerator0" (- (`KismetMathLibrary.Max` (`local.Mana`) 1) 1))
  (`/Game/RLDB/Blueprints/Core/BP_Card.OnThisCardModified` (`self.OwningCard`))
  (return))