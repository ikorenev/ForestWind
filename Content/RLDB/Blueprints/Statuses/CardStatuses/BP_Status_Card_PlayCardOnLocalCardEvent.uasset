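; Card status that auto-plays its owning card when a bound local card event fires.
; On BeginPlay it binds its gameplay tags to the owner's dispatcher hub.
; RunEvent announces AutoPlay on the global hub, then uses the card untargeted, skipping playable checks and consequences, with queued delays for pacing.
; Cards tagged KeepAfterAutoPlay get their post-use event temporarily swapped to ReturnToHand, then restored.
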(event `self.ReceiveBeginPlay`
  (`parent.ReceiveBeginPlay`)
  (`/Game/RLDB/Blueprints/Core/BP_DispatcherHubComponent.BindMultipleEventsToHub` (`.ReturnValue` (`self.GetOwnersDispatcherHub`)) self (`self.GameplayTags`)))

(event `/Game/RLDB/Blueprints/Interfaces/BPI_EventHolder.RunEvent`
  (params (EventTag :type "GameplayTag Structure") (CallingObject :type "Object Object Reference (by ref)") (bGlobal :type Boolean) (Payload :type "Object Object Reference (by ref)") (CallTags :type "GameplayTagContainer Structure (by ref)"))
  (bind _asbp_card (cast `/Game/RLDB/Blueprints/Core/BP_Card` (`self.GetOwner`)))
  (`/Game/RLDB/Blueprints/Libraries/BPFL_Singletons.QueueDelay` 0.4)
  (`/Game/RLDB/Blueprints/Libraries/BPFL_Singletons.QueueEventInGlobalDispatcherHub` (struct :`TagName` "Event.Action.AutoPlay") (`self.GetOwner`) null 1.0)
  (if (`BlueprintGameplayTagLibrary.HasTag` (`/Game/RLDB/Blueprints/Core/BP_Card.GetGameplayTags` _asbp_card) (struct :`TagName` "Flag.KeepAfterAutoPlay") true)
    (set `self.OriginalPostUseEvent` (`/Game/RLDB/Blueprints/Core/BP_Card.GetPostUseEvent` _asbp_card "NewEnumerator0"))
    (`/Game/RLDB/Blueprints/Core/BP_Card.SetPostUseEvent` _asbp_card "NewEnumerator0" (struct :`TagName` "Event.Card.ReturnToHand"))
    (`/Game/RLDB/Blueprints/Core/BP_Card.AttemptUseCardUntargeted` _asbp_card true true true)
    (`/Game/RLDB/Blueprints/Core/BP_Card.SetPostUseEvent` _asbp_card "NewEnumerator0" (`self.OriginalPostUseEvent`))
    (`/Game/RLDB/Blueprints/Libraries/BPFL_Singletons.QueueDelay` 1.0)
    (else
      (`/Game/RLDB/Blueprints/Core/BP_Card.AttemptUseCardUntargeted` _asbp_card true true true)
      (`/Game/RLDB/Blueprints/Libraries/BPFL_Singletons.QueueDelay` 1.0))))