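; BP_Status_ManaGain is a status that updates an actor's mana, apparently at turn start.
; It binds to the turn-start event on its owner's dispatcher hub and acts only if the calling actor has a BP_Status_Mana component.
; It broadcasts a global ManaGain event, increments StatusValue, clears any Interrupt flag, and passes StatusValue to the Mana component's SetStatusValue.
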(event `self.ReceiveBeginPlay`
  (`parent.ReceiveBeginPlay`)
  (`/Game/RLDB/Blueprints/Core/BP_DispatcherHubComponent.BindMultipleEventsToHub` (`.ReturnValue` (`self.GetOwnersDispatcherHub`)) self (struct :`GameplayTags` (struct :`(TagName` "Event.TurnStart")))))

(event `/Game/RLDB/Blueprints/Interfaces/BPI_EventHolder.RunEvent`
  (params (EventTag :type "GameplayTag Structure") (CallingObject :type "Object Object Reference (by ref)") (bGlobal :type Boolean) (Payload :type "Object Object Reference (by ref)") (CallTags :type "GameplayTagContainer Structure (by ref)"))
  (bind _statusvalue (`self.StatusValue`))
  (bind _asactor (cast `Actor` CallingObject))
  (bind _returnvalue (`Actor.GetComponentByClass` _asactor "/Game/RLDB/Blueprints/Statuses/BP_Status_Mana.BP_Status_Mana_C"))
  (if (`KismetSystemLibrary.IsValid` _returnvalue)
    (`|SwitchGameplayTag` EventTag
      (:`Event.TurnStart`
        (`/Game/RLDB/Blueprints/Libraries/BPFL_Singletons.CallEventInGlobalDispatcherHub` (struct :`TagName` "Event.ManaGain") self)
        (`/Engine/EditorBlueprintResources/StandardMacros.IncrementInt` _statusvalue
          (:`  `
            (if (`self.bInterrupt`)
              (set `self.bInterrupt` false))
            (`self.SetStatusValue` _returnvalue _statusvalue false false null)))))))