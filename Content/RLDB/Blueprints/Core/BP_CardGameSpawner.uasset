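; BP_CardGameSpawner sets up a card game encounter when play begins.
; It spawns the actors in SpawnOrderActors in array order at its own transform, then requests a game save through the GameInstance.
; It adds each persistent hero twice to the first BP_MinionTrack and fills the second from the current encounter's data table minion rows, relying on GetAllActorsOfClass order to tell the tracks apart.
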(event `self.ReceiveBeginPlay`
  (for _array_element (`self.SpawnOrderActors`)
    (`|SpawnActorFromClass` _array_element (`self.GetTransform`) "AlwaysSpawn" "SelectDefaultAtRuntime" null null))
  (message `/Game/RLDB/Blueprints/Interfaces/BPI_CardGameInstance.AttemptSaveGame` (`GameplayStatics.GetGameInstance`) "" false)
  (bind _outactors (`GameplayStatics.GetAllActorsOfClass` "/Game/RLDB/Blueprints/Core/BP_MinionTrack.BP_MinionTrack_C"))
  (bind _persistentheroes (message `/Game/RLDB/Blueprints/Interfaces/BPI_CardGameInstance.GetPersistentHeroesFromInstance` (`GameplayStatics.GetGameInstance`)))
  (for _array_element_2 _persistentheroes
    (bind _output (`|GetArrayItem` _outactors))
    (bind _returnvalue (`KismetArrayLibrary.Array_Length` (`/Game/RLDB/Blueprints/Core/BP_MinionTrack.Minions` _output)))
    (`/Game/RLDB/Blueprints/Core/BP_MinionTrack.AddMinionToTrack` _output _returnvalue _array_element_2 true)
    (`/Game/RLDB/Blueprints/Core/BP_MinionTrack.AddMinionToTrack` _output _returnvalue _array_element_2 true))
  (bind _currentencounter (message `/Game/RLDB/Blueprints/Interfaces/BPI_CardGameInstance.GetCurrentEncounterFromInstance` (`GameplayStatics.GetGameInstance`)))
  (for _array_element_3 (`.Minions_10_4F0922FD423311AB44916DAA1B6F80E1` (break `/Game/RLDB/Blueprints/Structs/FEncounter` _currentencounter))
    (bind _returnvalue_2 (`|GetDataTableRow` (break `DataTableRowHandle` _array_element_3) (`.RowName` (break `DataTableRowHandle` _array_element_3)))
      (:`then`
        (bind _output_2 (`|GetArrayItem` _outactors 1))
        (`/Game/RLDB/Blueprints/Core/BP_MinionTrack.AddMinionToTrack` _output_2 (`KismetArrayLibrary.Array_Length` (`/Game/RLDB/Blueprints/Core/BP_MinionTrack.Minions` _output_2)) _returnvalue_2 true)))))

(fn `UserConstructionScript`)