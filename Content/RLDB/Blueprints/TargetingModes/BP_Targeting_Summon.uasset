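; Card targeting mode that selects summons on the card owner's minion track whose gameplay tags match the card effect's tags.
; FindValidTargets replaces the parent logic, gathering all minions on the owner track and keeping those whose BP_GameplayTagComponent shares any exact tag with the effect.
; TargetsFound reflects whether the track holds any minions, even if none pass the tag filter.
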(fn `FindAllSummonsWithMatchingTags`
  (params (GameplayTags :type "GameplayTagContainer Structure (by ref)") (Minions :type "Array of /Game/RLDB/Blueprints/Core/BP_Minion Object Reference"))
  (returns (MatchingTargets :type "Array of Actor Object Reference"))
  (locals (LocalMatchingTargets :type "Array of Actor Object Reference"))
  (for _array_element Minions
    (bind _returnvalue (`Actor.GetComponentByClass` _array_element "/Game/RLDB/Blueprints/Core/BP_GameplayTagComponent.BP_GameplayTagComponent_C"))
    (`/Engine/EditorBlueprintResources/StandardMacros.IsValid` _returnvalue
      (:`Is Valid`
        (if (`BlueprintGameplayTagLibrary.HasAnyTags` GameplayTags (`/Game/RLDB/Blueprints/Core/BP_GameplayTagComponent.GameplayTags` _returnvalue) true)
          (`KismetArrayLibrary.Array_Add` (`local.LocalMatchingTargets`) _array_element)))))
  (return (`local.LocalMatchingTargets`)))

(fn `FindValidTargets`
  (params (SpecifiedTargets :type "Array of Actor Object Reference (by ref)") (CardEffect :type "/Game/RLDB/Blueprints/Structs/FCardEffect Structure") (Card :type "/Game/RLDB/Blueprints/Core/BP_Card Object Reference") (bPreview :type Boolean))
  (returns (bTargetsFound :type Boolean) (ValidTargets :type "Array of Actor Object Reference"))
  (bind (_bfoundanytargets _minions) (`self.GetAllMinionsOnOwnerTrack` Card))
  (bind _matchingtargets (`self.FindAllSummonsWithMatchingTags` (`.GameplayTags_24_CC3A96B84AC557056996C8A91DF06498` (break `/Game/RLDB/Blueprints/Structs/FCardEffect` CardEffect)) _minions))
  (return _bfoundanytargets _matchingtargets))

(fn `GetAllMinionsOnOwnerTrack`
  (params (Card :type "/Game/RLDB/Blueprints/Core/BP_Card Object Reference"))
  (returns (bFoundAnyTargets :type Boolean) (Minions :type "Array of /Game/RLDB/Blueprints/Core/BP_Minion Object Reference"))
  (bind _ownertrack (`self.FindMinionTracks` Card))
  (`/Engine/EditorBlueprintResources/StandardMacros.IsValid` _ownertrack
    (:`Is Valid`
      (bind _minions (`/Game/RLDB/Blueprints/Core/BP_MinionTrack.Minions` _ownertrack))
      (if (> (`KismetArrayLibrary.Array_Length` _minions) 0)
        (return true _minions)
        (else
          (return false))))
    (:`Is Not Valid`
      (return false))))