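; BP_Plate1 is a pressure plate that reacts to physics-simulating components inside its Box trigger.
; An overlap, including one already present at BeginPlay, passes a DoOnce gate to lower the Button and send ActivateMessage to a valid Observer.
; Any physics component leaving raises the Button, sends DeactivateMessage and resets the gate, without checking for remaining overlaps or Observer validity.
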(event `self.ReceiveBeginPlay`
  (bind _observer (`self.Observer`))
  (for _array_element (`PrimitiveComponent.GetOverlappingComponents` (`self.Box`))
    (if (`SceneComponent.IsSimulatingPhysics` _array_element "None")
      (`/Engine/EditorBlueprintResources/StandardMacros.IsValid` _observer :!label _label
        (:`Is Valid`
          (`/Engine/EditorBlueprintResources/StandardMacros.DoOnce` false :!label _label_2
            (:`Completed`
              (message `/Game/Blooming/Blueprints/BPI_Activate.Activate` _observer self)
              (`SceneComponent.K2_AddLocalOffset` (`self.Button`) (0.0 0.0 -6.0) false false))))))))

(event `self.Box.OnComponentBeginOverlap`
  (params (OverlappedComponent :type "PrimitiveComponent Object Reference") (OtherActor :type "Actor Object Reference") (OtherComp :type "PrimitiveComponent Object Reference") (OtherBodyIndex :type Integer) (bFromSweep :type Boolean) (SweepResult :type "HitResult Structure (by ref)"))
  (if (`SceneComponent.IsSimulatingPhysics` OtherComp "None")
    (goto _label)))

(event `self.Box.OnComponentEndOverlap`
  (params (OverlappedComponent :type "PrimitiveComponent Object Reference") (OtherActor :type "Actor Object Reference") (OtherComp :type "PrimitiveComponent Object Reference") (OtherBodyIndex :type Integer))
  (if (`SceneComponent.IsSimulatingPhysics` OtherComp "None")
    (`SceneComponent.K2_AddLocalOffset` (`self.Button`) (0.0 0.0 6.0) false false)
    (message `/Game/Blooming/Blueprints/BPI_Activate.Deactivate` (`self.Observer`) self)
    (goto _label_2 :!via `Reset`)))

(fn `UserConstructionScript`
  (`parent.UserConstructionScript`))